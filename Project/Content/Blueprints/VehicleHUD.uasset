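; Vehicle HUD that draws the speed and gear readouts for a MainCar pawn while its IsInCar flag is false.
; DrawHUD scales text position and size by the screen's ratio to 1280x720, keeping the layout proportional across resolutions.
; Speed and gear strings come straight from the owning pawn, with the gear color switching when the car is in reverse.
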(event EventDrawHUD
  (params (SizeX :type Integer) (SizeY :type Integer))
  ;[1 1 1] Calculate ratio from 720p
  (bind _asmain_car (Utilities|Casting|CastToMainCar (Class|HUD|GetOwningPawn)))
  (if (not (Variables|/Game/Blueprints/Sedan/MainCar.MainCar_C|GetIsInCar _asmain_car))
    (Utilities|FlowControl|Sequence
      (:then_0
        (Variables|Default|SetHUDXRatio (/ (Math|Conversions|ToFloat(Integer) SizeX) 1.28e+03)))
      (:then_1
        (Variables|Default|SetHUDYRatio (/ (Math|Conversions|ToFloat(Integer) SizeY) 7.2e+02)))
      (:then_2
        ;[1 1 1] Print vehicle speed
        (bind _asmain_car_2 (Utilities|Casting|CastToMainCar (Class|HUD|GetOwningPawn)))
        (HUD|DrawText (Variables|/Game/Blueprints/Sedan/MainCar.MainCar_C|GetSpeed%20Display%20String _asmain_car_2) "(R=1.000000,G=1.000000,B=1.000000,A=1.000000)" (* 805.0 (Variables|Default|GetHUDXRatio)) (* 455.0 (Variables|Default|GetHUDYRatio)) "/Engine/EngineFonts/RobotoDistanceField.RobotoDistanceField" (* 1.4 (Variables|Default|GetHUDYRatio)) false)
        ;[1 1 1] Print vehicle gear
        (bind _asmain_car_3 (Utilities|Casting|CastToMainCar (Class|HUD|GetOwningPawn)))
        (HUD|DrawText (Utilities|String|Append "Gear:" (Variables|/Game/Blueprints/Sedan/MainCar.MainCar_C|GetGear%20Display%20String _asmain_car_3)) (Math|Color|SelectColor (Variables|/Game/Blueprints/Sedan/MainCar.MainCar_C|GetGearDisplayReverseColor _asmain_car_3) (Variables|/Game/Blueprints/Sedan/MainCar.MainCar_C|GetGearDisplayColor _asmain_car_3) (Variables|/Game/Blueprints/Sedan/MainCar.MainCar_C|GetInReverseGear _asmain_car_3)) (* 805.0 (Variables|Default|GetHUDXRatio)) (* 5e+02 (Variables|Default|GetHUDYRatio)) "/Engine/EngineFonts/RobotoDistanceField.RobotoDistanceField" (* 1.4 (Variables|Default|GetHUDYRatio)) false) ; If True display Current Gear
      ))))

(fn ConstructionScript)