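; GameMode for a multiplayer game with a lobby, handling player joins and leaves, chat history, kicking and map travel.
; It keeps a list of player controllers, feeds each one the server info from the GameInstance and rebuilds every client's player list when the roster changes.
; Server messages go out through the first player controller, and logged chat is replayed to newcomers.
; It also creates game UI and teleports players to shuffled DefaultSpawn points.
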(event Custom|JoinGame
  (bind _returnvalue (Game|GetPlayerController 0))
  ;[1 1 1] Change Map
  (if (Utilities|Enum|Equal(Enum) (Variables|Default|GetServerMap) "Cars")
    (Development|ExecuteConsoleCommand "servertravel/Game/Maps/Cars" _returnvalue)
    (bind _asbp_game_instace (Utilities|Casting|CastToBP_GameInstace (Game|GetGameInstance) :!label _label))
    (Default|JoinGame _asbp_game_instace)
    (elif (Utilities|Enum|Equal(Enum) (Variables|Default|GetServerMap) "OriginalMap")
      (Development|ExecuteConsoleCommand "servertravel/Game/Maps/OriginalMap" _returnvalue)
      (goto _label))))

(event Custom|UpdateServer
  ;[1 1 1] Update Server
  (for _array_element (Variables|Default|GetAllPCs)
    (bind _asbp_player_controller (Utilities|Casting|CastToBP_PlayerController _array_element))
    (Default|ClearPlayerList _asbp_player_controller)
    (for (_array_element_2 _array_index) (Variables|Default|GetAllPCs)
      (Default|AddPlayer _asbp_player_controller (Utilities|Text|ToText(String) (Class|AdvancedSessionsLibrary|GetPlayerName _array_element_2)) _array_index)))
  (for _array_element_3 (Variables|Default|GetAllPCs)
    (bind _asbp_player_controller_2 (Utilities|Casting|CastToBP_PlayerController _array_element_3))
    (Default|UpdateNumberOfPlayers _asbp_player_controller_2 (Utilities|Array|Length (Variables|Default|GetAllPCs)))))

(event Custom|KickPlayer
  (params (Index :type Integer))
  ;[1 1 1] Kick Player
  (bind _asbp_player_controller (Utilities|Casting|CastToBP_PlayerController (Utilities|Array|Get(acopy) (Variables|Default|GetAllPCs) Index)))
  (Default|Kick _asbp_player_controller))

(event Custom|AddMessageToChatHistory
  (params (Data :type Chat%20Message%20Structure%20Structure))
  ;[1 1 1] Load Message History
  (Utilities|Array|Add (Variables|Default|GetMessageLOG) Data))

(event Custom|SendServerMessage
  (params (Message :type String))
  ;[1 1 1] Send Server Message
  (bind _asbp_player_controller (Utilities|Casting|CastToBP_PlayerController (Game|GetPlayerController 0)))
  (Default|AddMessagefromServertoEachPlayer _asbp_player_controller Message (Utilities|Struct|MakeSlateColor "(R=0.091657,G=0.191682,B=1.000000,A=1.000000)") true))

(event Custom|Continue
  ;[1 1 1] add each player controller to the list and update server
  (CallFunction|SendServerMessage (Utilities|String|Append (Class|AdvancedSessionsLibrary|GetPlayerName (stale EventPostLogin NewPlayer)) " has joined"))
  (Default|AddLobbyBPW (stale EventPostLogin _asbp_player_controller) (Variables|Default|GetServerName) (Variables|Default|GetServerMap) (Variables|Default|GetServerMode) (Variables|Default|GetServerSlots))
  (CallFunction|UpdateServer)
  ;[1 1 1] Load Message History
  (for _array_element (Variables|Default|GetMessageLOG)
    (bind _asbp_player_controller (Utilities|Casting|CastToBP_PlayerController (stale EventPostLogin NewPlayer)))
    (Default|AddMessagetoChat _asbp_player_controller _array_element)))

(event Custom|SetGamemode
  (params (GameMode :type Integer))
  ;[1 1 1] NewGameMode
  (Variables|Default|SetGameMode GameMode))

(event Custom|TeleportOnEachPlayer
  ;[1 1 1] Teleport each player
  (if (== (Variables|Default|GetGameMode) 1)
    (for (_array_element _array_index) (Variables|Default|GetAllPCs)
      (bind _asbp_player_controller (Utilities|Casting|CastToBP_PlayerController _array_element))
      (Default|TeleportonOwningClient _asbp_player_controller (Transformation|GetWorldLocation (Variables|/Game/Blueprints/SpawnPoint/DefaultSpawn.DefaultSpawn_C|GetSphere (Utilities|Array|Get(acopy) (Variables|Default|GetDefaultSpanPoints) _array_index)))))
    (elif (== (Variables|Default|GetGameMode) 1)
      _)))

(event Custom|CreateGameUIOnEachPlayer
  ;[1 1 1] Create Game UI
  (for _array_element (Variables|Default|GetAllPCs)
    (bind _asbp_player_controller (Utilities|Casting|CastToBP_PlayerController _array_element))
    (Default|CreateGameUI _asbp_player_controller)))

(event EventOnSwapPlayerControllers
  (params (OldPC :type Player%20Controller%20Object%20Reference) (NewPC :type Player%20Controller%20Object%20Reference))
  ;[1 1 1] NewGameMode
  (if (not (Variables|Default|GetTestMode))
    (Utilities|Array|Add (Variables|Default|GetPCsNeedToSetUp) NewPC)
    (Utilities|Array|Add (Variables|Default|GetAllPCs) NewPC)))

(event EventTick
  (params (DeltaSeconds :type Float%20%28single-precision%29)))

(event EventPostLogin
  (params (NewPlayer :type Player%20Controller%20Object%20Reference))
  ;[1 1 1] add each player controller to the list and update server
  (if (Variables|Default|GetTestMode)
    (Utilities|Array|Add (Variables|Default|GetPCsNeedToSetUp) NewPlayer)
    (Utilities|Array|Add (Variables|Default|GetAllPCs) NewPlayer)
    (else
      (Networking|SwitchHasAuthority
        (:Authority
          (Utilities|Array|Add (Variables|Default|GetAllPCs) NewPlayer)
          (bind _asbp_game_instace (Utilities|Casting|CastToBP_GameInstace (Game|GetGameInstance)))
          (Variables|Default|SetServerName (Variables|/Game/Blueprints/BP_GameInstace.BP_GameInstace_C|GetServerName _asbp_game_instace))
          (Variables|Default|SetServerMap (Variables|/Game/Blueprints/BP_GameInstace.BP_GameInstace_C|GetServerMap _asbp_game_instace))
          (Variables|Default|SetServerMode (Variables|/Game/Blueprints/BP_GameInstace.BP_GameInstace_C|GetServerMode _asbp_game_instace))
          (Variables|Default|SetServerSlots (Variables|/Game/Blueprints/BP_GameInstace.BP_GameInstace_C|GetServerSlots _asbp_game_instace))
          (bind _asbp_player_controller (Utilities|Casting|CastToBP_PlayerController NewPlayer))
          (Default|PlayerDataSetup _asbp_player_controller))))))

(event EventOnLogout
  (params (ExitingController :type Controller%20Object%20Reference))
  (bind _allpcs (Variables|Default|GetAllPCs))
  ;[1 1 1] Log Out of a player
  (bind (_array_element _array_index) (Utilities|Array|ForEachLoopwithBreak _allpcs :!label _label)
    (:LoopBody
      (if (== ExitingController _array_element)
        (CallFunction|SendServerMessage (Utilities|String|Append (Class|AdvancedSessionsLibrary|GetPlayerName _array_element) " has left"))
        (goto _label Break)))
    (:Completed
      (Utilities|Array|RemoveIndex _allpcs _array_index)
      (CallFunction|UpdateServer))))

(event EventBeginPlay
  ;[1 1 1] Begin Play
  (bind _outactors (Actor|GetAllActorsOfClass "/Game/Blueprints/SpawnPoint/DefaultSpawn.DefaultSpawn_C"))
  (bind _output_get (Variables|Default|SetDefaultSpanPoints _outactors))
  (Utilities|Array|Shuffle _output_get))

(fn ConstructionScript)