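; Game Instance Blueprint that handles multiplayer session hosting, player save data and the loading screen.
; CreateLobby stores server settings, publishes them as Advanced Session extra settings (password included), then opens the fixed DetailBuildingMap as listen server on success.
; JoinGame only destroys the current session.
; Save, load and exists-check functions persist LanName in a SaveGame slot, while show/hide events manage the loading widget.
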(event Custom|CreateLobby
  (params (ServerName :type String) (ServerMap :type String) (ServerSlots :type Integer) (ServerMode :type String) (ServerMethod_Lan? :type Boolean) (HasPassword? :type Boolean) (Password :type String))
  ;[1 1 1] Create Advanced Session
  (Variables|Default|SetServerName ServerName)
  (Variables|Default|SetServerMap ServerMap)
  (Variables|Default|SetServerSlots ServerSlots)
  (Variables|Default|SetServerMode ServerMode)
  (Variables|Default|SetServerMethod_Lan? ServerMethod_Lan?)
  (Variables|Default|SetHasPassword? HasPassword?)
  (Variables|Default|SetPassword Password)
  (|AdvancedSession (Utilities|Array|MakeArray (Class|AdvancedSessionsLibrary|MakeLiteralSessionPropertyString "NAME" (Variables|Default|GetServerName)) (Class|AdvancedSessionsLibrary|MakeLiteralSessionPropertyString "MAP" (Variables|Default|GetServerMap)) (Class|AdvancedSessionsLibrary|MakeLiteralSessionPropertyString "MODE" (Variables|Default|GetServerMode)) (Class|AdvancedSessionsLibrary|MakeLiteralSessionPropertyBool "LAN" (Variables|Default|GetServerMethod_Lan?)) (Class|AdvancedSessionsLibrary|MakeLiteralSessionPropertyBool "HASPASSWORD" (Variables|Default|GetHasPassword?)) (Class|AdvancedSessionsLibrary|MakeLiteralSessionPropertyString "PASSWORD" (Variables|Default|GetPassword))) (Game|GetPlayerController 0) (Variables|Default|GetServerSlots) 0 (Variables|Default|GetServerMethod_Lan?) true false true true false false false true
    (:OnSuccess
      (Game|OpenLevel(byName) "DetailBuildingMap" true "listen"))))

(event Custom|JoinGame
  ;[1 1 1] Join Game
  (|DestroySession (Game|GetPlayerController 0)))

(event Custom|SavePlayerData
  (params (Lan_Name :type String))
  ;[1 1 1] Save/Load Player Data
  (bind _output_get (Variables|Default|SetLan_Name Lan_Name))
  (bind _returnvalue (SaveGame|CreateSaveGameObject "/Game/Blueprints/SavePlayerData.SavePlayerData_C"))
  (Variables|/Game/Blueprints/SavePlayerData.SavePlayerData_C|SetLanName _returnvalue _output_get)
  (SaveGame|SaveGametoSlot _returnvalue (Variables|Default|GetPlayerSlotSG)))

(event Custom|LoadPlayerData
  ;[1 1 1] Save/Load Player Data
  (bind _returnvalue (SaveGame|LoadGamefromSlot (Variables|Default|GetPlayerSlotSG)))
  (bind _assave_player_data (Utilities|Casting|CastToSavePlayerData _returnvalue))
  (Variables|Default|SetLan_Name (Variables|/Game/Blueprints/SavePlayerData.SavePlayerData_C|GetLanName _assave_player_data)))

(event Custom|ShowLoadingScreen
  ;[1 1 1] LoadingScreen
  (bind _returnvalue (UserInterface|CreateWidget "/Game/UI/Widgets/BPW_LoadingScreen.BPW_LoadingScreen_C"))
  (bind _output_get (Variables|Default|SetLoadingWB _returnvalue))
  (UserInterface|Viewport|AddtoViewport _output_get 0))

(event Custom|HideLoadingScreen
  ;[1 1 1] LoadingScreen
  (Widget|RemovefromParent (Variables|Default|GetLoadingWB)))

(fn PlayerDataExists?
  (bind _returnvalue (SaveGame|DoesSaveGameExist (Variables|Default|GetPlayerSlotSG)))
  (return _returnvalue))